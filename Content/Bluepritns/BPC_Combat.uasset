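; Player combat component that handles target lock-on and sword combo attacks for BP_ThirdPersonCharacter.
; Lock input toggles a camera-forward sphere-traced target with an attached marker actor, while Tick aims control rotation at it.
; Attack input plays one combo montage, where notifies stop it unless another press is buffered.
; Begin/EndDamageTrace events run a looping timer that sphere-traces along the sword and applies damage, throttled by a DoOnce and delay.
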(event `self.ReceiveBeginPlay`
  ;[0.1451 0.1451 0.1451] Get Player
  (bind _asbp_third_person_character (cast `/Game/ThirdPerson/Blueprints/BP_ThirdPersonCharacter` (`self.GetOwner`)))
  (set `self.PlayerBP` _asbp_third_person_character))

(event `EnhancedInput|/Game/ThirdPerson/Input/Actions/IA_Lock`
  (params (ActionValue :type Boolean) (ElapsedSeconds :type "Float (double-precision)") (TriggeredSeconds :type "Float (double-precision)") (InputAction :type "InputAction Object Reference" :default "/Game/ThirdPerson/Input/Actions/IA_Lock.IA_Lock"))
  (bind _returnvalue (`Actor.GetTransform` (`self.TargetLockActor`)))
  (bind _transformcomponent (`PlayerCameraManager.TransformComponent` (`GameplayStatics.GetPlayerCameraManager` 0)))
  (bind (_returnvalue_x _returnvalue_y _returnvalue_z) (`KismetMathLibrary.BreakVector` (`SceneComponent.K2_GetComponentLocation` _transformcomponent)))
  (bind _returnvalue_2 (`KismetMathLibrary.MakeVector` _returnvalue_x _returnvalue_y (+ _returnvalue_z 25.0)))
  ;[0.1451 0.1451 0.1451] Find Target to Lock
  (:`Started`
    (`self.TargetLockActor`
      (:`then`
        ;;[0.1451 0.1451 0.1451] Unlock
        (set `self.TargetLockActor` null)
        (`/Game/ThirdPerson/Blueprints/BP_ThirdPersonCharacter.HandleMoveBackwards` (`self.PlayerBP`) true)
        (`Actor.K2_DestroyActor` (`self.TargetLockWidget`)))
      (:`else`
        (bind (_outhit _returnvalue_3) (`KismetSystemLibrary.SphereTraceSingleForObjects` :`Start` _returnvalue_2 :`End` (+ _returnvalue_2 (* (`KismetMathLibrary.GetForwardVector` (`SceneComponent.K2_GetComponentRotation` _transformcomponent)) 10000.0)) :`Radius` 150.0 :`ObjectTypes` (`|MakeArray` "ObjectTypeQuery3" :!type "EObjectTypeQuery Enum") :`DrawDebugType` "ForDuration" :`DrawTime` 2.0))
        (if _returnvalue_3
          (set `self.TargetLockActor` (`.HitActor` (`GameplayStatics.BreakHitResult` _outhit)))
          (`/Game/ThirdPerson/Blueprints/BP_ThirdPersonCharacter.HandleMoveBackwards` (`self.PlayerBP`) false)
          ;;[0.1451 0.1451 0.1451] Lock UI
          (bind _returnvalue_4 (`|SpawnActorFromClass` "/Game/Bluepritns/BP_TargetLockWidget.BP_TargetLockWidget_C" (`KismetMathLibrary.MakeTransform` (`KismetMathLibrary.MakeVector` (.x (.location _returnvalue)) (.y (.location _returnvalue)) (+ (.z (.location _returnvalue)) 20.0)) (.rotation _returnvalue)) "AlwaysSpawn" "MultiplyWithRoot" null null))
          (bind _output_get (set `self.TargetLockWidget` _returnvalue_4))
          (`Actor.K2_AttachToActor` _output_get (`self.TargetLockActor`) "None" "SnapToTarget" "SnapToTarget" "SnapToTarget" true))))))

(event `self.ReceiveTick`
  (params (DeltaSeconds :type "Float (single-precision)"))
  (bind _playerbp (`self.PlayerBP`))
  ;[0.1451 0.1451 0.1451] Update camera to locked target
  (bind _targetlockactor (`self.TargetLockActor`)
    (:`then`
      (bind (_returnvalue_roll _returnvalue_pitch _returnvalue_yaw) (`KismetMathLibrary.BreakRotator` (`KismetMathLibrary.FindLookAtRotation` (`Actor.K2_GetActorLocation` _playerbp) (`Actor.K2_GetActorLocation` _targetlockactor))))
      (`Controller.SetControlRotation` (`Pawn.GetController` _playerbp) (`KismetMathLibrary.MakeRotator` _returnvalue_roll (+ _returnvalue_pitch -20.0) _returnvalue_yaw)))
    (:`else`)))

(event `EnhancedInput|/Game/ThirdPerson/Input/Actions/IA_Attack`
  (params (ActionValue :type Boolean) (ElapsedSeconds :type "Float (double-precision)") (TriggeredSeconds :type "Float (double-precision)") (InputAction :type "InputAction Object Reference" :default "/Game/ThirdPerson/Input/Actions/IA_Attack.IA_Attack"))
  ;[0.1451 0.1451 0.1451] Sword Combo Animation
  (:`Started`
    (if (not (`self.IsAttacking`))
      (set `self.IsAttacking` true)
      (`|PlayMontage` (`Character.Mesh` (`self.PlayerBP`)) "/Game/Characters/Souls/Combat/SwordAttackCombo_Montage.SwordAttackCombo_Montage"
        (:`OnCompleted`
          (set `self.IsAttacking` false :!label _label)
          (set `self.Combo` false :!label _label_2))
        (:`OnInterrupted`
          (goto _label))
        (:`OnNotifyBegin`
          (if (and (`self.IsAttacking`) (`self.Combo`))
            (goto _label_2)
            (else
              (`AnimInstance.Montage_Stop` (`SkeletalMeshComponent.GetAnimInstance` (`Character.Mesh` (`self.PlayerBP`))) 0.2 "/Game/Characters/Souls/Combat/SwordAttackCombo_Montage.SwordAttackCombo_Montage")
              (set `self.IsAttacking` false)
              (set `self.Combo` false)))))
      (else
        (set `self.Combo` true)))))

(event `End Damage Trace`
  ;[0.1451 0.1451 0.1451] Attack Trace
  (if (`KismetSystemLibrary.K2_IsValidTimerHandle` (stale `Begin Damage Trace` _returnvalue))
    (`KismetSystemLibrary.K2_ClearAndInvalidateTimerHandle` (stale `Begin Damage Trace` _returnvalue))))

(event `Begin Damage Trace`
  ;[0.1451 0.1451 0.1451] Attack Trace
  (bind _returnvalue (`KismetSystemLibrary.K2_SetTimerDelegate` (delegate `Damage Trace`) 0.01 true)))

(event `Damage Trace`
  (bind _playerbp (`self.PlayerBP`))
  ;[0.1451 0.1451 0.1451] Attack Trace
  (bind (_outhit _returnvalue) (`KismetSystemLibrary.SphereTraceSingleForObjects` :`Start` (`SceneComponent.K2_GetComponentLocation` (`/Game/ThirdPerson/Blueprints/BP_ThirdPersonCharacter.Start Sword Trace Pos` _playerbp)) :`End` (`SceneComponent.K2_GetComponentLocation` (`/Game/ThirdPerson/Blueprints/BP_ThirdPersonCharacter.End Sword Trace Pos` _playerbp)) :`Radius` 25.0 :`ObjectTypes` (`|MakeArray` "ObjectTypeQuery3" :!type "EObjectTypeQuery Enum") :`DrawDebugType` "ForOneFrame"))
  (if _returnvalue
    (`/Engine/EditorBlueprintResources/StandardMacros.DoOnce` false :!label _label_3
      (:`Completed`
        (`GameplayStatics.ApplyDamage` (`.HitActor` (`GameplayStatics.BreakHitResult` _outhit)) (`self.SwordDamage`))
        (`KismetSystemLibrary.Delay` 0.3)
        (goto _label_3 :!via `Reset`)))))